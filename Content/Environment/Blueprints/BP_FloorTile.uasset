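; BP_FloorTile is a self-replacing track segment for an endless runner, also used behind the start menu camera.
; When the runner or menu camera overlaps EndTrigger, it has BP_GameMode add a tile, plays explosion effects on it, then destroys itself after a delay.
; After the first second of game time, construction adds difficulty-based blockers at random points, plus an occasional jump obstacle that may bring a pickup.
; GetAttachTransform exposes the tile's attach point.
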(event OnComponentBeginOverlap(EndTrigger)
  (params (OtherActor :type Actor%20Object%20Reference) (OtherComp :type Primitive%20Component%20Object%20Reference) (OtherBodyIndex :type Integer) (bFromSweep :type Boolean) (SweepResult :type Hit%20Result%20Structure%20%28by%20ref%29))
  ;[1 1 1] Create new floor tile on overlap event of any tile
  (Utilities|Casting|CastToBP_RunnerCharacter OtherActor
    (:then
      _)
    (:CastFailed
      (Utilities|Casting|CastToBP_StartMenu_Camera OtherActor)))
  (bind _asbp_game_mode (Utilities|Casting|CastToBP_GameMode (Game|GetGameMode)))
  (bind _floor_tile (Default|AddFloorTile _asbp_game_mode))
  ;[1 1 1] Floor tile creation effect
  (for _array_element (Variables|Default|GetAttachEffectPoints)
    (Effects|SpawnEmitterAttached "/Game/Environment/Particles/P_Explosion.P_Explosion" (VehicleSound|GetRootComponent _floor_tile) "None" _array_element))
  (Audio|SpawnSoundAttached "/Game/Environment/Audio/Explosion01.Explosion01" (VehicleSound|GetRootComponent _floor_tile) "None" _array_element "0, 0, 0" "KeepRelativeOffset" true 0.1 0.1)
  ;[1 1 1] Cleanup old floor tiles
  (Utilities|FlowControl|Delay 2.0)
  (Actor|DestroyActor))

(fn ConstructionScript
  (CallFunction|SetSpawnPoints)
  (if (> (Utilities|Time|GetGameTimeinSeconds) 1.0)
    (CallFunction|SpawnBlocker)
    ;[1 1 1] Spawn jump obstacle
    (switch int (Math|Random|RandomIntegerinRange 0 5)
      (:0
        (CallFunction|SpawnObstacleJump)
        ;[1 1 1] Spawn pickup
        (switch int (Math|Random|RandomIntegerinRange 0 5)
          (:0
            (CallFunction|SpawnPickup)))))))

(fn SetSpawnPoints
  ;[1 1 1] Get all spawn points relative transforms
  (Variables|Default|SetSpawnPoints (Utilities|Array|MakeArray (Transformation|GetRelativeTransform (Variables|Default|GetSpawnPoint_FrontMid)) (Transformation|GetRelativeTransform (Variables|Default|GetSpawnPoint_FrontLeft)) (Transformation|GetRelativeTransform (Variables|Default|GetSpawnPoint_FrontRight)) (Transformation|GetRelativeTransform (Variables|Default|GetSpawnPoint_BackMid)) (Transformation|GetRelativeTransform (Variables|Default|GetSpawnPoint_BackLeft)) (Transformation|GetRelativeTransform (Variables|Default|GetSpawnPoint_BackRight))))
  (Variables|Default|SetAttachEffectPoints (Utilities|Array|MakeArray (Variables|/Script/Engine.SceneComponent|GetRelativeLocation (Variables|Default|GetAttachEffectPoint_Right)) (Variables|/Script/Engine.SceneComponent|GetRelativeLocation (Variables|Default|GetAttachEffectPoint_Left)) (Variables|/Script/Engine.SceneComponent|GetRelativeLocation (Variables|Default|GetAttachEffectPoint_Mid))))
  (Variables|Default|SetSpawnPickupPoints (Utilities|Array|MakeArray (Transformation|GetRelativeTransform (Variables|Default|GetSpawnPoint_Pickup_Mid)) (Transformation|GetRelativeTransform (Variables|Default|GetSpawnPoint_Pickup_Right)) (Transformation|GetRelativeTransform (Variables|Default|GetSpawnPoint_Pickup_Left)))))

(fn SpawnBlocker
  (bind _spawnpoints (Variables|Default|GetSpawnPoints))
  (bind _asbp_game_mode (Utilities|Casting|CastToBP_GameMode (Game|GetGameMode)))
  (if (>= (Variables|/Game/BP_GameMode.BP_GameMode_C|GetDifficulty _asbp_game_mode) 2)
    (for _index (range 0 1)
      (AddComponent|AddChildActorComponent false (Utilities|Array|Get(acopy) _spawnpoints (Math|Random|RandomIntegerinRange 0 (Utilities|Array|LastIndex _spawnpoints)))))
    (else
      (for _index_2 (range 0 (Variables|/Game/BP_GameMode.BP_GameMode_C|GetDifficulty _asbp_game_mode))
        (AddComponent|AddChildActorComponent false (Utilities|Array|Get(acopy) _spawnpoints (Math|Random|RandomIntegerinRange 0 (Utilities|Array|LastIndex _spawnpoints))))))))

(fn SpawnObstacleJump
  (bind _asbp_game_mode (Utilities|Casting|CastToBP_GameMode (Game|GetGameMode)))
  (if (>= (Variables|/Game/BP_GameMode.BP_GameMode_C|GetDifficulty _asbp_game_mode) 2)
    (for _index (range 0 (Variables|/Game/BP_GameMode.BP_GameMode_C|GetDifficulty _asbp_game_mode))
      (AddComponent|AddChildActorComponent false (Transformation|GetRelativeTransform (Variables|Default|GetSpawnPoint_ObstacleJump))))
    (else
      (AddComponent|AddChildActorComponent false (Transformation|GetRelativeTransform (Variables|Default|GetSpawnPoint_ObstacleJump))))))

(fn SpawnPickup
  (bind _spawnpickuppoints (Variables|Default|GetSpawnPickupPoints))
  (AddComponent|AddChildActorComponent false (Utilities|Array|Get(acopy) _spawnpickuppoints (Math|Random|RandomIntegerinRange 0 (Utilities|Array|LastIndex _spawnpickuppoints)))))

(fn GetAttachTransform
  ;[1 1 1] Get world transform of the attach point
  (return (Transformation|GetWorldTransform (Variables|Default|GetAttachPoint))))