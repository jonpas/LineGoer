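; Player character for an endless runner that constantly moves forward along world axes, with sideways steering, jumping, shooting and pausing.
; A Dead flag blocks movement, jump and fire, while JumpPressed is exposed for animations.
; Firing works only when not falling, spawning a zero-rotation BP_Projectile at the weapon's Muzzle socket and using a short Delay to destroy it.
; The pause input toggles game pause and writes a Paused variable.
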(event EventTick
  (params (DeltaSeconds :type Float%20%28single-precision%29))
  ;[1 1 1] Movement
  ;;[1 1 1] Endless forward movement
  (if (not (Variables|Default|GetDead))
    (Pawn|Input|AddMovementInput (Math|Vector|GetForwardVector "0, 0, 0") 1.0 false)))

(event Input|ActionEvents|InputActionFire
  (params (Key :type Key%20Structure :default "AnyKey"))
  (bind _weapon (Variables|Default|GetWeapon))
  (bind _returnvalue (Transformation|GetSocketTransform _weapon "Muzzle" "RTS_World"))
  (bind (_location _rotation _scale) (Math|Transform|BreakTransform _returnvalue))
  ;[1 1 1] Fire
  (:Pressed
    (if (not (or (AI|Components|NavMovement|IsFalling (Variables|Character|GetCharacterMovement)) (Variables|Default|GetDead)))
      (bind _returnvalue_2 (Game|SpawnActorfromClass "/Game/Character/Weapon/Blueprints/BP_Projectile.BP_Projectile_C" (Math|Transform|MakeTransform _location "0, 0, 0" _scale) "Undefined" 0 0))
      ;;[1 1 1] Cleanup old projectiles
      (Utilities|FlowControl|Delay 1.0)
      (Actor|DestroyActor _returnvalue_2))))

(event Input|ActionEvents|InputActionJump
  (params (Key :type Key%20Structure :default "AnyKey"))
  ;[1 1 1] Jump (set variable for animations)
  (:Pressed
    (if (not (Variables|Default|GetDead))
      (Character|Jump)
      (Variables|Default|SetJumpPressed true)))
  (:Released
    (Variables|Default|SetJumpPressed false)))

(event Input|ActionEvents|InputActionPause
  (params (Key :type Key%20Structure :default "AnyKey"))
  (bind _returnvalue (Game|IsGamePaused))
  (bind _returnvalue_2 (not _returnvalue))
  ;[1 1 1] Pause
  (:Pressed
    (Game|SetGamePaused _returnvalue_2)
    (Variables|Default|SetPaused _returnvalue_2)))

(event Input|AxisEvents|InputAxisMoveRight
  (params (AxisValue :type Float%20%28single-precision%29))
  ;[1 1 1] Movement
  ;;[1 1 1] Left/Right movement on input
  (if (not (Variables|Default|GetDead))
    (Pawn|Input|AddMovementInput (Math|Vector|GetRightVector "0, 0, 0") AxisValue false)))

(fn ConstructionScript)