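; BP_Weapon is a weapon actor that a BP_Character_01 picks up by overlapping it and then fires.
; Pickup snaps it to the character mesh's Weapon socket and enables input on it for a player controller.
; The Fire input spawns a BP_Projectile at the skeletal mesh's Muzzle socket.
; The player index lookup feeding that controller choice sits on unconnected nodes, so it never executes.
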(event EventActorBeginOverlap
  (params (OtherActor :type Actor%20Object%20Reference))
  ;[1 1 1] Pickup
  (bind _asbp_character_01 (Utilities|Casting|CastToBP_Character_01 OtherActor))
  (Class|Actor|AttachRootComponentto (Variables|/Script/Engine.Character|GetMesh _asbp_character_01) "Weapon" "SnapToTargetIncludingScale" true)
  (Input|EnableInput (Game|GetPlayerController (stale _playerindex))))

(event Input|ActionEvents|InputActionFire
  (params (Key :type Key%20Structure :default "AnyKey"))
  ;[1 1 1] Fire
  (:Pressed
    (Game|SpawnActorfromClass "/Game/Character/Weapon/Blueprints/BP_Projectile.BP_Projectile_C" (Transformation|GetSocketTransform (Variables|Default|GetSkeletalMesh) "Muzzle" "RTS_World") "Undefined" 0 0)))

(fn ConstructionScript)